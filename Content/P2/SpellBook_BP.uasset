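; SpellBook_BP is a pickup in a side-scroller that grants the player a spell when the SideScrollerCharacter overlaps it.
; On pickup it plays a sound, destroys itself and switches on Type to call NewSpell on the character.
; The Open Doors and Magic Wheel types also trigger their linked MagicObject, opening the door or starting the wheel's first movement, while Levitation only grants the spell.
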(event EventBeginPlay
  (bind _output_get (Variables|Default|SetInitial%20Location (Transformation|GetActorLocation)))
  (Variables|Default|SetDestination%20Location (+ _output_get "0, 0,40.000000")))

(event Collision|EventActorBeginOverlap
  (params (OtherActor :type Actor%20Object%20Reference))
  (bind _asside_scroller_character (Utilities|Casting|CastToSideScrollerCharacter OtherActor))
  (Audio|PlaySoundatLocation "/Game/P2/Sounds/PickABook.PickABook" (Variables|Default|GetInitial%20Location) "0, 0, 0" 0.6 1.0 0.0 0 0 0)
  (Variables|Default|SetIsPicked true)
  (Actor|DestroyActor)
  (switch Utilities|FlowControl|Switch|SwitchonBooksType (Variables|Default|GetType)
    (:NewEnumerator0
      (bind _asmagic_door_bp (Utilities|Casting|CastToMagicDoor_BP (Variables|Default|GetMagicObject)))
      (Default|OpenIt _asmagic_door_bp)
      (Default|NewSpell _asside_scroller_character "Open Door 
"))
    (:NewEnumerator1
      (bind _asmagic_wheel_bp (Utilities|Casting|CastToMagicWheel_BP (Variables|Default|GetMagicObject)))
      (Default|FirstMovement _asmagic_wheel_bp)
      (Default|NewSpell _asside_scroller_character "Magic Wheel 
"))
    (:NewEnumerator3
      (Default|NewSpell _asside_scroller_character "Levitation 
"))))

(fn ConstructionScript)