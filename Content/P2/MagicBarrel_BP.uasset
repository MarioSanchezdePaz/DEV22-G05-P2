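; Levitatable barrel pawn that the player possesses and flies into a cart for delivery.
; StartLevitating takes possession, axis inputs move it sideways and vertically, and E returns control to the main character.
; Hitting the cart snaps and attaches the barrel, disables mesh collision, notifies the cart and releases control.
; Other hits tint it red and spend a hit; running out resets it to spawn and releases control.
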(event Custom|StartLevitating
  (Variables|Default|SetPossesed true)
  (Pawn|Possess (Game|GetPlayerController 0) self))

(event Custom|ControlBack
  (Pawn|Possess (Game|GetPlayerController 0) (Variables|Default|GetMainCharacter)))

(event EventBeginPlay
  (Variables|Default|SetSpawn (Transformation|GetActorLocation))
  (Variables|Default|SetCompletedBarrels 0))

(event Collision|EventHit
  (params (MyComp :type Primitive%20Component%20Object%20Reference) (Other :type Actor%20Object%20Reference) (OtherComp :type Primitive%20Component%20Object%20Reference) (bSelfMoved :type Boolean) (HitLocation :type Vector :default "0, 0, 0") (HitNormal :type Vector :default "0, 0, 0") (NormalImpulse :type Vector :default "0, 0, 0") (Hit :type Hit%20Result%20Structure%20%28by%20ref%29))
  (if (not (Variables|Default|GetIsPlaced))
    (Utilities|Casting|CastToCart_Pawn Other
      (:then
        (Transformation|SetActorLocation "1320.000000,2880.000000,175.000000" false false)
        (Collision|SetCollisionEnabled (Variables|Default|GetBarrelMesh) "NoCollision")
        (Development|PrintString "Has entregado un barril!")
        (Audio|PlaySoundatLocation "/Game/P2/Sounds/DeliverBarrel.DeliverBarrel" "1320.000000,3060.000000,70.000000" "0, 0, 0" 1.0 1.0 0.0 0 0 0)
        (Transformation|AttachActorToActor self (Variables|Default|GetpawnRef) "" "KeepRelative" "KeepRelative" "KeepRelative" true)
        (Variables|Default|SetIsPlaced true)
        (Default|IncomingBarrel (Variables|Default|GetpawnRef))
        (CallFunction|ControlBack))
      (:CastFailed
        (bind _returnvalue (Rendering|Material|CreateDynamicMaterialInstance (Variables|Default|GetBarrelMesh) 0 0 "None" :!class /Script/Engine.PrimitiveComponent))
        (Rendering|Material|SetVectorParameterValue _returnvalue "Basecolor Tint" "(R=0.921875,G=0.029333,B=0.000000,A=1.000000)" :!class /Script/Engine.MaterialInstanceDynamic)
        (bind _output_get (Variables|Default|SetHitsLeft (- (Variables|Default|GetHitsLeft) 1)))
        (Utilities|FlowControl|Delay 1.0)
        (if (not (> _output_get 0))
          (Transformation|SetActorRelativeLocation self (Variables|Default|GetSpawn))
          (Variables|Default|SetHitsLeft 3)
          (Rendering|Material|SetVectorParameterValue _returnvalue "Basecolor Tint" "(R=1.000000,G=1.000000,B=1.000000,A=1.000000)" :!class /Script/Engine.MaterialInstanceDynamic)
          (CallFunction|ControlBack))))))

(event Input|AxisEvents|InputAxisMoveRight
  (params (AxisValue :type Float%20%28single-precision%29))
  (Pawn|Input|AddMovementInput "0.000000,-1.000000,0.000000" AxisValue false))

(event Input|AxisEvents|InputAxisMoveUp
  (params (AxisValue :type Float%20%28single-precision%29))
  (Pawn|Input|AddMovementInput "0, 0,1.000000" AxisValue false))

(event Input|KeyboardEvents|E
  (params (Key :type Key%20Structure :default "None"))
  (:Pressed
    (Variables|Default|SetPossesed false)
    (CallFunction|ControlBack)))

(fn ConstructionScript)